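; BP_CierreExperiencia runs the timed ending of the experience, driven by the per-second event of BP_RelojInterno.
; At one configured second it plays a clock-ticking sound with timeline-driven volume.
; At the activation second it plays a voice or sound cue, then a door-opening sequence.
; From the final second it attaches a VR sign to the player camera, plays music and quits after a delay.
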(event `ComprobarCierre`
  (params (SegundoExacto :type Integer))
  (if (== SegundoExacto (`self.NewVar`))
    (bind _returnvalue (`GameplayStatics.SpawnSoundAtLocation` "/Game/Sonidos/dragon-studio-slow-cinematic-clock-ticking-357979.dragon-studio-slow-cinematic-clock-ticking-357979" (`self.K2_GetActorLocation`) (struct) 1.0 1.0 0.0 null null))
    (bind (_direction _newtrack_0) (`Timeline|SubidaTicTac`)
      (:`Update`
        (`AudioComponent.SetVolumeMultiplier` _returnvalue _newtrack_0)))
    (elif (== SegundoExacto (`self.SegundoDeActivacion`))
      (`/Engine/EditorBlueprintResources/StandardMacros.DoOnce` false
        (:`Completed`
          (`GameplayStatics.PlaySoundAtLocation` "/Game/Sonidos/A_Hello.A_Hello" (`self.K2_GetActorLocation`) (struct) 1.0 1.0 0.0 null null null null)
          (`KismetSystemLibrary.Delay` 1.0)
          (bind (_outactor _returnvalue_2) (`LevelSequencePlayer.CreateLevelSequencePlayer` "/Game/Sequencers/S_PuertaAbrir.S_PuertaAbrir"))
          (`MovieSceneSequencePlayer.Play` _returnvalue_2)))
      (elif (>= SegundoExacto (`self.SegundoFinal`))
        (`/Engine/EditorBlueprintResources/StandardMacros.DoOnce` false
          (:`Completed`
            (bind _returnvalue_3 (`|SpawnActorFromClass` "/Game/BP/BP_FinJuego/BP_CartelVR.BP_CartelVR_C" (`KismetMathLibrary.MakeTransform` (0.0 0.0 0.0)) "Undefined" "MultiplyWithRoot" null null))
            (bind _returnvalue_4 (`self.K2_AttachToComponent` _returnvalue_3 (`PlayerCameraManager.TransformComponent` (`GameplayStatics.GetPlayerCameraManager` 0)) "None" "SnapToTarget" "KeepRelative" "KeepRelative" true))
            (`self.K2_SetActorRelativeLocation` (100.0 0.0 0.0) _returnvalue_4)
            (`GameplayStatics.PlaySound2D` "/Game/Sonidos/A_CancionMotivacion.A_CancionMotivacion" 1.0 1.0 10.0 null null)
            (`KismetSystemLibrary.Delay` 7.0)
            (`KismetSystemLibrary.QuitGame` null "Quit")))))))

(event `self.ReceiveBeginPlay`
  (bind _returnvalue (`GameplayStatics.GetActorOfClass` "/Game/BP/BP_RelojInterno/BP_RelojInterno.BP_RelojInterno_C"))
  (add `/Game/BP/BP_RelojInterno/BP_RelojInterno.AlPasarUnSegundo` _returnvalue (delegate `ComprobarCierre`)))

(fn `UserConstructionScript`)