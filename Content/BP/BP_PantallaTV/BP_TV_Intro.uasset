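; TV screen actor that shows timed hint messages on its W_PantallaTV widget as the room's clock advances.
; It binds to BP_RelojInterno's per-second dispatcher and sends indexed texts from TextosPistas at fixed seconds, most after a notification sound and delay.
; A looping timer types each message letter by letter until complete.
; After the second message, the Amanecer timeline drives the intensity of all PointLight actors.
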(event `AñadirLetra`
  (bind _output (`|GetArrayItem` (`self.TextosPistas`) (`self.IndiceActual`)))
  (set `self.ContadorLetras` (+ (`self.ContadorLetras`) 1))
  (bind _asw_pantalla_tv (cast `/Game/Widget/W_PantallaTV` (`WidgetComponent.GetUserWidgetObject` (`self.Widget`))))
  (`TextBlock.SetText` (`/Game/Widget/W_PantallaTV.TextoInstrucciones` _asw_pantalla_tv) (`KismetTextLibrary.Conv_StringToText` (`KismetStringLibrary.GetSubstring` _output 0 (`self.ContadorLetras`))))
  (if (>= (`self.ContadorLetras`) (`KismetStringLibrary.Len` _output))
    (`KismetSystemLibrary.K2_ClearAndInvalidateTimerHandle` (`self.TimerLetras`))))

(event `self.ReceiveBeginPlay`
  (bind _returnvalue (`GameplayStatics.GetActorOfClass` "/Game/BP/BP_RelojInterno/BP_RelojInterno.BP_RelojInterno_C"))
  (add `/Game/BP/BP_RelojInterno/BP_RelojInterno.AlPasarUnSegundo` _returnvalue (delegate `EventosDeLaSala`))
  (bind _returnvalue_2 (`KismetSystemLibrary.K2_SetTimerDelegate` (delegate `AñadirLetra`) 0.04 true :!label _label))
  (set `self.TimerLetras` _returnvalue_2))

(event `EventosDeLaSala`
  (params (SegundoExacto :type Integer))
  (bind _returnvalue (`KismetMathLibrary.Conv_IntToDouble` (`self.DelayMensajes`)))
  (if (== SegundoExacto 0)
    (`self.MandarMensaje` 0)
    (elif (== SegundoExacto 1)
      (`GameplayStatics.PlaySoundAtLocation` "/Game/Sonidos/Sonido_Notificacion_TV.Sonido_Notificacion_TV" (`self.K2_GetActorLocation`) (struct) 1.0 1.0 0.0 null null null null)
      (`KismetSystemLibrary.Delay` _returnvalue)
      (`self.MandarMensaje` 1)
      (`KismetSystemLibrary.Delay` 5.0)
      (bind _outactors (`GameplayStatics.GetAllActorsOfClass` "/Script/Engine.PointLight"))
      (set `self.MisLuces` _outactors)
      (bind (_direction _fuerza_de_luz) (`Timeline|Amanecer` :!via `PlayFromStart`)
        (:`Update`
          (for _array_element (`self.MisLuces`)
            (`LightComponent.SetIntensity` (`PointLight.PointLightComponent` _array_element) _fuerza_de_luz))))
      (elif (== SegundoExacto 59)
        (`GameplayStatics.PlaySoundAtLocation` "/Game/Sonidos/Sonido_Notificacion_TV.Sonido_Notificacion_TV" (`self.K2_GetActorLocation`) (struct) 1.0 1.0 0.0 null null null null)
        (`KismetSystemLibrary.Delay` _returnvalue)
        (`self.MandarMensaje` 2)
        (elif (== SegundoExacto 119)
          (`GameplayStatics.PlaySoundAtLocation` "/Game/Sonidos/Sonido_Notificacion_TV.Sonido_Notificacion_TV" (`self.K2_GetActorLocation`) (struct) 1.0 1.0 0.0 null null null null)
          (`KismetSystemLibrary.Delay` _returnvalue)
          (`self.MandarMensaje` 3)
          (elif (== SegundoExacto 179)
            (`GameplayStatics.PlaySoundAtLocation` "/Game/Sonidos/Sonido_Notificacion_TV.Sonido_Notificacion_TV" (`self.K2_GetActorLocation`) (struct) 1.0 1.0 0.0 null null null null)
            (`KismetSystemLibrary.Delay` _returnvalue)
            (`self.MandarMensaje` 4)
            (elif (== SegundoExacto 239)
              (`GameplayStatics.PlaySoundAtLocation` "/Game/Sonidos/Sonido_Notificacion_TV.Sonido_Notificacion_TV" (`self.K2_GetActorLocation`) (struct) 1.0 1.0 0.0 null null null null)
              (`KismetSystemLibrary.Delay` _returnvalue)
              (`self.MandarMensaje` 5)
              (elif (== SegundoExacto 299)
                (`GameplayStatics.PlaySoundAtLocation` "/Game/Sonidos/Sonido_Notificacion_TV.Sonido_Notificacion_TV" (`self.K2_GetActorLocation`) (struct) 1.0 1.0 0.0 null null null null)
                (`KismetSystemLibrary.Delay` _returnvalue)
                (`self.MandarMensaje` 6)
                (elif (== SegundoExacto 330)
                  (`GameplayStatics.PlaySoundAtLocation` "/Game/Sonidos/Sonido_Notificacion_TV.Sonido_Notificacion_TV" (`self.K2_GetActorLocation`) (struct) 1.0 1.0 0.0 null null null null)
                  (`KismetSystemLibrary.Delay` _returnvalue)
                  (`self.MandarMensaje` 7))))))))))

(event `MandarMensaje`
  (params (NumeroDeFrase :type Integer))
  (set `self.IndiceActual` NumeroDeFrase)
  (set `self.ContadorLetras` 0)
  (goto _label))

(fn `UserConstructionScript`)