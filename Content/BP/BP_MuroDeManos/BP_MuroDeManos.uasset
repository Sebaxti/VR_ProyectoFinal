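; BP_MuroDeManos is a wall-of-hands actor that triggers its animation sequence at a set time on the game's internal clock.
; The construction script rebuilds 30 MisManos instances at random points inside the ZonaDeAparicion box, all sharing one fixed rotation.
; On BeginPlay it binds to BP_RelojInterno's per-second event.
; Once SegundoDeActivacion is reached, a DoOnce plays the S_MuroDeManos level sequence.
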(event `VerificarTiempo`
  (params (SegundoExacto :type Integer))
  (if (>= SegundoExacto (`self.SegundoDeActivacion`))
    (`/Engine/EditorBlueprintResources/StandardMacros.DoOnce` false
      (:`Completed`
        (bind (_outactor _returnvalue) (`LevelSequencePlayer.CreateLevelSequencePlayer` "/Game/Sequencers/S_MuroDeManos.S_MuroDeManos" (`self.Settings`)))
        (`MovieSceneSequencePlayer.Play` _returnvalue)))))

(event `self.ReceiveBeginPlay`
  (bind _returnvalue (`GameplayStatics.GetActorOfClass` "/Game/BP/BP_RelojInterno/BP_RelojInterno.BP_RelojInterno_C"))
  (add `/Game/BP/BP_RelojInterno/BP_RelojInterno.AlPasarUnSegundo` _returnvalue (delegate `VerificarTiempo`)))

(fn `UserConstructionScript`
  (bind _zonadeaparicion (`self.ZonaDeAparicion`))
  (`InstancedStaticMeshComponent.ClearInstances` (`self.MisManos`))
  (for _ (range 1 31)
    (`InstancedStaticMeshComponent.AddInstance` (`self.MisManos`) (`KismetMathLibrary.MakeTransform` (`KismetMathLibrary.RandomPointInBoundingBox` (`SceneComponent.RelativeLocation` _zonadeaparicion) (`BoxComponent.GetScaledBoxExtent` _zonadeaparicion)) (struct :`Pitch` 180.0 :`Roll` 90.0)) false)))