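; Danger zone for the VR pawn that darkens the player's view with a radial vignette, intensifying toward the zone's center.
; It listens to BP_RelojInterno's per-second event until a configured second, then enables the effect and unbinds.
; Overlap adds a dynamic M_RadialVignette blendable to the pawn's camera.
; Tick drives its darkness with a cubic distance falloff, and leaving the zone resets it to zero.
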(event `ComprobarTiempoEfecto`
  (params (SegundoExacto :type Integer))
  (if (>= SegundoExacto (`self.SegundoInicioEfecto`))
    (set `self.EfectoHabilitado` true)
    (remove `/Game/BP/BP_RelojInterno/BP_RelojInterno.AlPasarUnSegundo` (stale `self.ReceiveBeginPlay` _returnvalue) (delegate `ComprobarTiempoEfecto`))))

(event `self.ReceiveBeginPlay`
  (bind _returnvalue (`GameplayStatics.GetActorOfClass` "/Game/BP/BP_RelojInterno/BP_RelojInterno.BP_RelojInterno_C"))
  (add `/Game/BP/BP_RelojInterno/BP_RelojInterno.AlPasarUnSegundo` _returnvalue (delegate `ComprobarTiempoEfecto`)))

(event `self.ReceiveTick`
  (params (DeltaSeconds :type "Float (single-precision)"))
  (if (`self.EfectoHabilitado`)
    (`/Engine/EditorBlueprintResources/StandardMacros.IsValid` (`self.PlayerPrefab`)
      (:`Is Valid`
        (`MaterialInstanceDynamic.SetScalarParameterValue` (`self.VigneteInstance`) "IntensidadOscuridad" (* (`KismetMathLibrary.MultiplyMultiply_FloatFloat` (`KismetMathLibrary.MapRangeClamped` (`KismetMathLibrary.Vector_Distance` (`SceneComponent.K2_GetComponentLocation` (`/Game/VRTemplate/Blueprints/VRPawn.Camera` (`self.PlayerPrefab`))) (`self.K2_GetActorLocation`)) 0.0 300.0 1.0) 3.0) 15.0))))))

(event `self.ZonaDePeligro.OnComponentBeginOverlap`
  (params (OverlappedComponent :type "PrimitiveComponent Object Reference") (OtherActor :type "Actor Object Reference") (OtherComp :type "PrimitiveComponent Object Reference") (OtherBodyIndex :type Integer) (bFromSweep :type Boolean) (SweepResult :type "HitResult Structure (by ref)"))
  (bind _asvrpawn (cast `/Game/VRTemplate/Blueprints/VRPawn` OtherActor))
  (set `self.PlayerPrefab` _asvrpawn)
  (bind _returnvalue (`KismetMaterialLibrary.CreateDynamicMaterialInstance` "/Game/BP/BP_ZonaDePeligro/M_RadialVignette.M_RadialVignette" "IntensidadOscuridad"))
  (set `self.VigneteInstance` _returnvalue)
  (`CameraComponent.AddOrUpdateBlendable` (`/Game/VRTemplate/Blueprints/VRPawn.Camera` (`self.PlayerPrefab`)) (`self.VigneteInstance`) 1.0))

(event `self.ZonaDePeligro.OnComponentEndOverlap`
  (params (OverlappedComponent :type "PrimitiveComponent Object Reference") (OtherActor :type "Actor Object Reference") (OtherComp :type "PrimitiveComponent Object Reference") (OtherBodyIndex :type Integer))
  (cast `/Game/VRTemplate/Blueprints/VRPawn` OtherActor)
  (`MaterialInstanceDynamic.SetScalarParameterValue` (`self.VigneteInstance`) "IntensidadOscuridad" 0.0)
  (set `self.PlayerPrefab` null))

(fn `UserConstructionScript`)