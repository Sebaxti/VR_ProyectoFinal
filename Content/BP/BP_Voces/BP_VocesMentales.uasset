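; BP_VocesMentales triggers the "mental voices" sound that plays in the player's head once a set moment in the game is reached.
; On BeginPlay it finds BP_RelojInterno and binds to its per-second event, comparing each second against SegundoDeActivacion.
; A DoOnce then attaches A_SonidoEsquizo to the player camera, and the SubidaParanoia timeline drives its volume multiplier.
; A camera-relative behind-left offset calculation is left unconnected.
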(event `ComprobarVoces`
  (params (SegundoExacto :type Integer))
  (if (>= SegundoExacto (`self.SegundoDeActivacion`))
    (`/Engine/EditorBlueprintResources/StandardMacros.DoOnce` false
      (:`Completed`
        (bind _returnvalue (`GameplayStatics.SpawnSoundAttached` "/Game/Sonidos/A_SonidoEsquizo.A_SonidoEsquizo" (`PlayerCameraManager.TransformComponent` (`GameplayStatics.GetPlayerCameraManager` 0)) "None" (-20.0 -30.0 0.0) (struct) "KeepRelativeOffset" false 1.0 1.0 0.0 "/Game/Audio/ATT_SalaTV.ATT_SalaTV" null))
        (bind (_direction _newtrack_0) (`Timeline|SubidaParanoia`)
          (:`Update`
            (`AudioComponent.SetVolumeMultiplier` _returnvalue _newtrack_0)))))))

(event `self.ReceiveBeginPlay`
  (bind _returnvalue (`GameplayStatics.GetActorOfClass` "/Game/BP/BP_RelojInterno/BP_RelojInterno.BP_RelojInterno_C"))
  (add `/Game/BP/BP_RelojInterno/BP_RelojInterno.AlPasarUnSegundo` _returnvalue (delegate `ComprobarVoces`)))

(fn `UserConstructionScript`)